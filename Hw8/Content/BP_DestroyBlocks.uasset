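; BP_DestroyBlocks is a breakable block that reacts to hits from BP_Ball.
; Each ball hit decrements a Hit counter, and while hits remain the cube switches to a different material to show damage.
; When the counter runs out, the block destroys itself and randomly spawns a BP_Bonus at its transform.
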(event `self.ReceiveHit`
  (params (MyComp :type "PrimitiveComponent Object Reference") (Other :type "Actor Object Reference") (OtherComp :type "PrimitiveComponent Object Reference") (bSelfMoved :type Boolean) (HitLocation :type "Vector Structure") (HitNormal :type "Vector Structure") (NormalImpulse :type "Vector Structure") (Hit :type "HitResult Structure (by ref)"))
  (cast `/Game/BP_Ball` Other)
  (bind _output_get (set `self.Hit` (- (`self.Hit`) 1)))
  (if (<= _output_get 0)
    (`self.K2_DestroyActor`)
    (if (`KismetMathLibrary.RandomBool`)
      (`|SpawnActorFromClass` "/Game/BP_Bonus.BP_Bonus_C" (`self.GetTransform`) "Undefined" "OverrideRootScale" null null))
    (else
      (`PrimitiveComponent.SetMaterial` (`self.Cube`) 0 "/Engine/MapTemplates/Materials/BasicAsset03.BasicAsset03"))))

(fn `UserConstructionScript`)