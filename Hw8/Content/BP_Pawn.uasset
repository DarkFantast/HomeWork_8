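; Player pawn for a ball game that slides sideways, launches balls and collects bonuses.
; MoveRight input applies fixed, swept local X offsets per call, opposite in sign to the axis and not scaled by delta time.
; SpawnBall runs on BeginPlay and on each BP_Bonus pickup, which destroys the bonus.
; It spawns a BP_Ball at the capsule, stores it as PlayingBall and binds its OnDead event.
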(event `InputAxis|MoveRight`
  (params (AxisValue :type "Float (single-precision)"))
  (if (< AxisValue 0.0)
    (bind _sweephitresult (`self.K2_AddActorLocalOffset` (50.0 0.0 0.0) true))
    (if (`GameplayStatics.BreakHitResult` _sweephitresult)
      _)))

(event `InputAxis|MoveRight`
  (params (AxisValue :type "Float (single-precision)"))
  (if (> AxisValue 0.0)
    (bind _sweephitresult (`self.K2_AddActorLocalOffset` (-50.0 0.0 0.0) true))
    (if (`GameplayStatics.BreakHitResult` _sweephitresult)
      _)))

(event `self.ReceiveBeginPlay`
  (`self.SpawnBall`))

(event `self.ReceiveActorBeginOverlap`
  (params (OtherActor :type "Actor Object Reference"))
  (bind _asbp_bonus (cast `/Game/BP_Bonus` OtherActor))
  (`self.K2_DestroyActor` _asbp_bonus)
  (`self.SpawnBall`))

(event `self.ReceiveTick`
  (params (DeltaSeconds :type "Float (single-precision)")))

(fn `SpawnBall`
  (bind _returnvalue (`|SpawnActorFromClass` "/Game/BP_Ball.BP_Ball_C" (`KismetMathLibrary.MakeTransform` (`SceneComponent.K2_GetComponentLocation` (`self.Capsule`))) "AlwaysSpawn" "OverrideRootScale" null null))
  (bind _output_get (set `self.PlayingBall` _returnvalue))
  (add `/Game/BP_Ball.OnDead` _output_get (`|CreateDelegate` :!event `SpawnBall`))
  (return))

(fn `UserConstructionScript`)