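; BP_BlocksGenerator is an actor that builds a flat grid of BP_DestroyBlocks when play begins.
; Nested loops over X and Y spawn one block per cell, offset from the generator's location by the index times Padding along the world X and Y axes.
; All logic runs once in BeginPlay, with no construction script, tick or overlap behavior.
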(event `self.ReceiveBeginPlay`
  (for _index (range (+ (`self.X`) 1))
    (for _index_2 (range (+ (`self.Y`) 1))
      (`|SpawnActorFromClass` "/Game/BP_DestroyBlocks.BP_DestroyBlocks_C" (`KismetMathLibrary.MakeTransform` (+ (`self.K2_GetActorLocation`) (`KismetMathLibrary.MakeVector` (* _index (`self.Padding`)) (* _index_2 (`self.Padding`))))) "Undefined" "OverrideRootScale" null null))))

(fn `UserConstructionScript`)